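; BP_DialogCube is a trigger actor that opens a dialogue UI when something overlaps its Box component.
; On overlap it clears all widgets, creates WB_Dialogue_UI for player 0 and passes its Script variable in as the widget's TextList.
; It then shows the mouse cursor and switches input to Game and UI, focused on the dialogue widget.
; The overlap is not filtered by actor, so any overlapping object triggers the dialogue.
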(event OnComponentBeginOverlap(Box)
  (params (OverlappedComponent :type Primitive%20Component%20Object%20Reference) (OtherActor :type Actor%20Object%20Reference) (OtherComp :type Primitive%20Component%20Object%20Reference) (OtherBodyIndex :type Integer) (bFromSweep :type Boolean) (SweepResult :type Hit%20Result%20Structure%20%28by%20ref%29))
  (CallFunction|DisplayDialogUI1))

(event Custom|Display%20Dialog%20UI%201
  (bind _returnvalue (Game|GetPlayerController 0))
  (Viewport|RemoveAllWidgets)
  (bind _returnvalue_2 (UserInterface|CreateWidget "/Game/UI/WB_Dialogue_UI.WB_Dialogue_UI_C" (Game|GetPlayerController 0)))
  (UserInterface|Viewport|AddtoViewport _returnvalue_2 0)
  (Variables|/Game/UI/WB_Dialogue_UI.WB_Dialogue_UI_C|SetTextList _returnvalue_2 (Variables|Default|GetScript))
  (Variables|/Script/Engine.PlayerController|SetbShowMouseCursor _returnvalue true)
  (Input|SetInputModeGameandUI _returnvalue _returnvalue_2 "DoNotLock" true))

(event EventBeginPlay)

(event Collision|EventActorBeginOverlap
  (params (OtherActor :type Actor%20Object%20Reference)))

(event EventTick
  (params (DeltaSeconds :type Float%20%28single-precision%29)))

(fn ConstructionScript)