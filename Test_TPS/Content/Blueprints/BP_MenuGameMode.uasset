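; Menu game mode that shows the WB_MainMenu widget and cycles the background view through level actors tagged "Camera".
; A self-repeating switch event fades out, sets the next view target, starts its motion, fades back in and waits, wrapping around the list.
; A timeline nudges the active camera along its local Y on every update, accumulating the offset and undoing it when finished.
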(event Custom|Switch_Camera
  (CameraFades|StartCameraFade :self (Game|GetPlayerCameraManager 0) :ToAlpha 1.0 :Duration 0.4 :bHoldWhenFinished true)
  (Utilities|FlowControl|Delay 0.7)
  (Game|Player|SetViewTargetwithBlend (Game|GetPlayerController 0) (Utilities|Array|Get(acopy) (Variables|Default|GetCameraList) (Variables|Default|GetCurrent%20Camera%20Index)) 0.0 "VTBlend_Linear" 0.0 false)
  (CallFunction|CameraMovement (.AsCamera%20Actor (Utilities|Casting|CastToCameraActor (Utilities|Array|Get(acopy) (Variables|Default|GetCameraList) (Variables|Default|GetCurrent%20Camera%20Index)))))
  (CameraFades|StartCameraFade :self (Game|GetPlayerCameraManager 0) :FromAlpha 1.0 :Duration 0.7 :bHoldWhenFinished true)
  (Utilities|FlowControl|Delay 3.0)
  (bind _result (Math|Integer|IncrementInt (Variables|Default|GetCurrent%20Camera%20Index))
    (:%20%20
      (if (>= _result (Utilities|Array|Length (Variables|Default|GetCameraList)))
        (Variables|Default|SetCurrent%20Camera%20Index 0))
      (CallFunction|SwitchCamera))))

(event Custom|Camera_Movement
  (params (Camera :type Camera%20Actor%20Object%20Reference))
  (Timeline|타임라인_0 PlayFromStart
    (:Update
      (Transformation|AddActorLocalOffset Camera "0.000000,1.000000,0.000000" false false)
      (Variables|Default|SetCamera%20Moved%20Distance (+ (Variables|Default|GetCamera%20Moved%20Distance) "0,1.000000, 0")))
    (:Finished
      (Transformation|AddActorLocalOffset Camera (- "0, 0, 0" (Variables|Default|GetCamera%20Moved%20Distance)) false false)
      (Variables|Default|SetCamera%20Moved%20Distance "0, 0, 0"))))

(event EventBeginPlay
  (bind _returnvalue (UserInterface|CreateWidget "/Game/UI/WB_MainMenu.WB_MainMenu_C" (Game|GetPlayerController 0)))
  (UserInterface|Viewport|AddtoViewport _returnvalue 0)
  (bind _outactors (Actor|GetAllActorswithTag "Camera"))
  (bind _output_get (Variables|Default|SetCameraList _outactors))
  (if (> (Utilities|Array|Length _output_get) 0)
    (CallFunction|SwitchCamera)))

(event EventTick
  (params (DeltaSeconds :type Float%20%28single-precision%29)))

(fn ConstructionScript)